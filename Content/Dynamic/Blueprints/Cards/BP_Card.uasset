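; Card actor for a networked card game, holding its info, owning player index and slot index, with a text label showing name and HP.
; Click and unclick events swap the mesh material.
; Setting HP rebuilds the CardInfo struct and refreshes the label, which the CardInfo RepNotify also refreshes on replication.
; The attack event, owner and slot RepNotifies, and local slot lookup are empty stubs, and debug prints remain.
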(event Custom|SetHP_1
  (params (HP :type Integer))
  (bind _cardinfo (Variables|Default|GetCardInfo))
  (bind (_staticmesh _hp _damage _name) (Utilities|Struct|BreakS_CardInfo _cardinfo))
  (|SetBy-RefVar (Variables|Default|GetCardInfo) (Utilities|Struct|MakeS_CardInfo _staticmesh HP _damage _name))
  (CallFunction|UpdateVisuals))

(event EventBeginPlay
  (if (Pawn|IsLocalPlayerController (Game|GetPlayerController 0))
    (bind _asbp_pc_player_controller (Utilities|Casting|CastToBP_PC_PlayerController (Game|GetPlayerController 0)))
    (Variables|Default|SetAs%20BP%20PC%20Player%20Controller _asbp_pc_player_controller)
    (Development|PrintString "HI I AM CARD")))

(event EventCardClicked
  (Rendering|Material|SetMaterial (Variables|Default|GetCardMesh) 0 "/Engine/MapTemplates/Materials/BasicAsset01.BasicAsset01"))

(event EventCardUnclicked
  (Rendering|Material|SetMaterial (Variables|Default|GetCardMesh) 0 "/Engine/BasicShapes/BasicShapeMaterial.BasicShapeMaterial"))

(event EventCardAttack
  (params (Attacker :type Actor%20Object%20Reference) (Target :type Actor%20Object%20Reference)))

(event EventUpdateVisuals
  (CallFunction|RefreshVisuals))

(event EventSetCardInfo
  (params (CardInfo :type S%20Card%20Info%20Structure))
  (Variables|Default|SetCardInfo CardInfo))

(fn ConstructionScript
  (bind _cardinfo (Variables|Default|GetCardInfo))
  (bind (_staticmesh _hp _damage _name) (Utilities|Struct|BreakS_CardInfo _cardinfo))
  (Rendering|Components|TextRender|SetText (Variables|Default|GetTextRender) (Utilities|Text|ToText(String) (Utilities|String|Append (Utilities|String|ToString(Name) _name) "  " "" "  HP: " (Utilities|String|ToString(Integer) _hp)))))

(fn OnRepCardOwnerIndex)

(fn OnRepSlotIndex)

(fn GetLocalSlotIndex)

(fn OnRepCardInfo
  (CallFunction|RefreshVisuals))

(fn RefreshVisuals
  (bind _cardinfo (Variables|Default|GetCardInfo))
  (bind (_staticmesh _hp _damage _name) (Utilities|Struct|BreakS_CardInfo _cardinfo))
  (Rendering|Components|TextRender|SetText (Variables|Default|GetTextRender) (Utilities|Text|ToText(String) (Utilities|String|Append (Utilities|String|ToString(Name) _name) "  " "" "  HP: " (Utilities|String|ToString(Integer) _hp))))
  (Development|PrintString (Utilities|String|Append "CardNewHP" (Utilities|String|ToString(Integer) _hp))))

(fn GetCardInfo
  (return (Variables|Default|GetCardInfo)))

(fn GetOwnerPlayerIndex
  (bind _owningplayerindex (Variables|Default|GetOwningPlayerIndex))
  (Development|PrintString (Utilities|String|ToString(Integer) _owningplayerindex))
  (return _owningplayerindex))

(fn GetSlotIndex
  (return (Variables|Default|GetCardSlotIndex)))