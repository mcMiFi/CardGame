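; BP_CardDraftPosition is a card draft actor that displays two cards and captures them as textures.
; Each card is a child actor that receives its card info and refreshes its visuals through message calls.
; The construction script gives each of two scene captures its own runtime render target.
; RepNotifies on the two card infos refresh the matching card and create a dynamic material fed by its render target.
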(event EventBeginPlay)

(fn ConstructionScript
  (bind _displayedcard1 (Variables|Default|GetDisplayedCard1))
  (bind _displayedcard (Variables|Default|GetDisplayedCard))
  (bind _childactor (Variables|/Script/Engine.ChildActorComponent|GetChildActor _displayedcard1))
  (bind _childactor_2 (Variables|/Script/Engine.ChildActorComponent|GetChildActor _displayedcard))
  (Class|BPICardInterract|SetCardInfo(Message) _childactor_2 (Variables|Default|GetCardInfo1))
  (Class|BPICardInterract|UpdateVisuals(Message) _childactor_2)
  (Class|BPICardInterract|SetCardInfo(Message) _childactor (Variables|Default|GetCardInfo2))
  (Class|BPICardInterract|UpdateVisuals(Message) _childactor)
  (bind _returnvalue (Rendering|CreateRenderTarget2D 400 600 "RTF_RGBA16f"))
  (bind _output_get (Variables|Default|SetRenderTarget1 _returnvalue))
  (Variables|/Script/Engine.SceneCaptureComponent2D|SetTextureTarget (Variables|Default|GetSceneCaptureComponent2D1) _output_get)
  (bind _returnvalue_2 (Rendering|CreateRenderTarget2D 400 600 "RTF_RGBA16f"))
  (bind _output_get_2 (Variables|Default|SetRenderTarget2 _returnvalue_2))
  (Variables|/Script/Engine.SceneCaptureComponent2D|SetTextureTarget (Variables|Default|GetSceneCaptureComponent2D2) _output_get_2))

(fn OnRepCardInfo1
  (bind _displayedcard (Variables|Default|GetDisplayedCard))
  (bind _childactor (Variables|/Script/Engine.ChildActorComponent|GetChildActor _displayedcard))
  (Class|BPICardInterract|SetCardInfo(Message) _childactor (Variables|Default|GetCardInfo1))
  (Class|BPICardInterract|UpdateVisuals(Message) _childactor)
  (bind _returnvalue (Rendering|Material|CreateDynamicMaterialInstance "/Game/Static/Materials/RenderTargets/NewTextureRenderTarget2D_Mat.NewTextureRenderTarget2D_Mat" "None" "None" :!class /Script/Engine.KismetMaterialLibrary))
  (bind _output_get (Variables|Default|SetCardMat1 _returnvalue))
  (Rendering|Material|SetTextureParameterValue _output_get "CardTexture" (Variables|Default|GetRenderTarget1)))

(fn OnRepCardInfo2
  (bind _displayedcard1 (Variables|Default|GetDisplayedCard1))
  (bind _childactor (Variables|/Script/Engine.ChildActorComponent|GetChildActor _displayedcard1))
  (Class|BPICardInterract|SetCardInfo(Message) _childactor (Variables|Default|GetCardInfo2))
  (Class|BPICardInterract|UpdateVisuals(Message) _childactor)
  (bind _returnvalue (Rendering|Material|CreateDynamicMaterialInstance "/Game/Static/Materials/RenderTargets/NewTextureRenderTarget2D_2Card_Mat.NewTextureRenderTarget2D_2Card_Mat" "None" "None" :!class /Script/Engine.KismetMaterialLibrary))
  (bind _output_get (Variables|Default|SetCardMat2 _returnvalue))
  (Rendering|Material|SetTextureParameterValue _output_get "CardTexture" (Variables|Default|GetRenderTarget2)))