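; Game mode for a multiplayer card game that spawns the shared table on BeginPlay.
; It tracks connected player controllers through login, controller swap and logout, reassigning each player state's index by array position on every login.
; A SpawnPlayer helper spawns and possesses a pawn at a found PlayerStart but is not called here.
; Card spawning and initial dealing are empty stubs, and the game state cast only prints debug text.
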(event Custom|MC_SpawnCards)

(event EventBeginPlay
  (CallFunction|StartGame))

(event EventPostLogin
  (params (NewPlayer :type Player%20Controller%20Object%20Reference))
  (bind _asbp_pc_player_controller (Utilities|Casting|CastToBP_PC_PlayerController NewPlayer))
  (Utilities|Array|Add (Variables|Default|GetConnectedPlayersControllers) _asbp_pc_player_controller)
  (for (_array_element _array_index) (Variables|Default|GetConnectedPlayersControllers)
    (bind _asbp_ps_player_state (Utilities|Casting|CastToBP_PS_PlayerState (Variables|/Script/Engine.Controller|GetPlayerState _array_element)))
    (bind _output_get (Variables|/Game/Dynamic/Blueprints/Player/BP_PS_PlayerState.BP_PS_PlayerState_C|SetPlayerIndex _asbp_ps_player_state _array_index))
    (Development|PrintString (Utilities|String|ToString(Integer) _output_get))))

(event EventOnSwapPlayerControllers
  (params (OldPC :type Player%20Controller%20Object%20Reference) (NewPC :type Player%20Controller%20Object%20Reference))
  (bind _asbp_pc_player_controller (Utilities|Casting|CastToBP_PC_PlayerController NewPC))
  (Utilities|Array|Add (Variables|Default|GetConnectedPlayersControllers) _asbp_pc_player_controller))

(event EventOnLogout
  (params (ExitingController :type Controller%20Object%20Reference))
  (bind _asbp_pc_player_controller (Utilities|Casting|CastToBP_PC_PlayerController ExitingController))
  (Utilities|Array|RemoveItem (Variables|Default|GetConnectedPlayersControllers) _asbp_pc_player_controller))

(fn ConstructionScript)

(fn SpawnPlayer
  (params (PlayerController :type BP%20PC%20Player%20Controller%20Object%20Reference))
  (bind _returnvalue (Actor|GetActorOfClass "/Script/Engine.PlayerStart"))
  (bind _returnvalue_2 (Game|SpawnActorfromClass "/Game/Dynamic/Blueprints/Player/BP_P_Player.BP_P_Player_C" (Transformation|GetActorTransform _returnvalue) "Undefined" "MultiplyWithRoot" 0 0))
  (Pawn|Possess PlayerController _returnvalue_2)
  (Development|PrintString "PlayerSpawned"))

(fn GiveInitialCards
  (params (PlayerController :type BP%20PC%20Player%20Controller%20Object%20Reference))
  (for _index (range 0 3)
    _))

(fn StartGame
  (bind _returnvalue (Game|SpawnActorfromClass "/Game/Dynamic/Blueprints/Table/BP_Table.BP_Table_C" (LocalVariables|GetTableTransform) "Undefined" "MultiplyWithRoot" 0 0))
  (Variables|Default|SetBP_Table _returnvalue)
  (bind _asbp_gs_game_state (Utilities|Casting|CastToBP_GS_GameState (Game|GetGameState))
    (:then
      (Development|PrintString (Utilities|GetDisplayName _asbp_gs_game_state)))
    (:CastFailed
      (Development|PrintString "CastFailed"))))