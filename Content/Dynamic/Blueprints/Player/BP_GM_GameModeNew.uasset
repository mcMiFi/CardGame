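; Game mode for a two-player turn-based card battle that runs setup, attacks, turn order and the win check.
; Looping timers wait for two ready players to spawn the table, then two table-ready signals to deal shuffled DataTable cards into its slots and pick a random first player.
; Attack requests from the player to move subtract HP, empty dead slots and mark attackers moved.
; The index-based attack path also passes turns and ends the game.
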(event Custom|PlayerReady
  (params (ReadyPlayerController :type BP%20PC%20Player%20Controller%20Object%20Reference))
  (bind _asbp_ps_player_state (Utilities|Casting|CastToBP_PS_PlayerState (Variables|/Script/Engine.Controller|GetPlayerState ReadyPlayerController)))
  (Variables|/Game/Dynamic/Blueprints/Player/BP_PC_PlayerController.BP_PC_PlayerController_C|SetAs%20BP%20PS%20Player%20State ReadyPlayerController _asbp_ps_player_state)
  (Variables|/Game/Dynamic/Blueprints/Player/BP_PS_PlayerState.BP_PS_PlayerState_C|SetPlayerIndex _asbp_ps_player_state (Utilities|Array|Length (Variables|Default|GetReadyPlayers)))
  (Utilities|FlowControl|Delay 1.0)
  (Utilities|Array|Add (Variables|Default|GetReadyPlayers) ReadyPlayerController))

(event Custom|TableReady
  (Math|Integer|IncrementInt (Variables|Default|GetReadyTables)))

(event Custom|ManageCardAttackRequest
  (params (Attacker :type Actor%20Object%20Reference) (Reciever :type Actor%20Object%20Reference) (AttackingPlayerController :type BP%20PC%20Player%20Controller%20Object%20Reference))
  (if (== AttackingPlayerController (Variables|Default|GetPlayerToMove))
    (CallFunction|ManageCardAttack Attacker Reciever)))

(event Custom|ManageRequestCardAttack
  (params (AttackerCardIndex :type Integer) (RecieverCardIndex :type Integer) (RequestingPC :type BP%20PC%20Player%20Controller%20Object%20Reference))
  (if (== RequestingPC (Variables|Default|GetPlayerToMove))
    (CallFunction|ManageAttackCard AttackerCardIndex RecieverCardIndex)))

(event EventBeginPlay
  (Utilities|Time|SetTimerbyFunctionName 0 "CheckBothPlayersReady" 0.02 true)
  (Utilities|Time|SetTimerbyFunctionName 0 "CheckTablesReady" 0.02 true))

(event EventPostLogin
  (params (NewPlayer :type Player%20Controller%20Object%20Reference))
  (bind _asbp_pc_player_controller (Utilities|Casting|CastToBP_PC_PlayerController NewPlayer))
  (Utilities|Array|Add (Variables|Default|GetConnectedPlayersControllers) _asbp_pc_player_controller))

(event EventOnSwapPlayerControllers
  (params (OldPC :type Player%20Controller%20Object%20Reference) (NewPC :type Player%20Controller%20Object%20Reference))
  (bind _asbp_pc_player_controller (Utilities|Casting|CastToBP_PC_PlayerController NewPC))
  (Utilities|Array|Add (Variables|Default|GetConnectedPlayersControllers) _asbp_pc_player_controller))

(event EventOnLogout
  (params (ExitingController :type Controller%20Object%20Reference))
  (bind _asbp_pc_player_controller (Utilities|Casting|CastToBP_PC_PlayerController ExitingController))
  (Utilities|Array|RemoveItem (Variables|Default|GetConnectedPlayersControllers) _asbp_pc_player_controller))

(fn ConstructionScript)

(fn StartGame
  (bind _bp_gamestate_ref (Variables|Default|GetBP_GameState%20Ref))
  (bind _tableref (Variables|/Game/Dynamic/Blueprints/Player/BP_GS_GameState.BP_GS_GameState_C|GetTableRef _bp_gamestate_ref))
  (bind _slotsinfo (Variables|/Game/Dynamic/Blueprints/Table/BP_Table.BP_Table_C|GetSlotsInfo _tableref))
  (bind _outrownames (DataTable|GetDataTableRowNames (Variables|Default|GetDT_Cards)))
  (bind _output_get (Variables|Default|SetNonUsedCards _outrownames))
  (Utilities|Array|Shuffle _output_get)
  (CallFunction|SetupPlayer0Cards)
  (CallFunction|SetupPlayer1Cards)
  (for (_ _array_index) _slotsinfo
    (if (> _array_index 3)
      (bind _returnvalue (Utilities|GetDataTableRow (Variables|Default|GetDT_Cards) (Utilities|Array|Get(acopy) (Variables|Default|GetPlayer1Cards) (- _array_index 4)))
        (:then
          (Utilities|Array|SetArrayElem _slotsinfo _array_index (Utilities|Struct|MakeS_SlotInfo _array_index 1 true (Utilities|Struct|MakeS_CardInfo (.StaticMesh (Utilities|Struct|BreakS_CardInfo _returnvalue)) (.HP (Utilities|Struct|BreakS_CardInfo _returnvalue)) (.Damage (Utilities|Struct|BreakS_CardInfo _returnvalue)) (.Name (Utilities|Struct|BreakS_CardInfo _returnvalue)))))
          (Development|PrintString (Utilities|String|ToString(Name) (Utilities|Array|Get(acopy) (Variables|Default|GetPlayer1Cards) (- _array_index 4))))))
      (else
        (bind _returnvalue_2 (Utilities|GetDataTableRow (Variables|Default|GetDT_Cards) (Utilities|Array|Get(acopy) (Variables|Default|GetPlayer0Cards) _array_index))
          (:then
            (Utilities|Array|SetArrayElem _slotsinfo _array_index (Utilities|Struct|MakeS_SlotInfo _array_index 0 true (Utilities|Struct|MakeS_CardInfo (.StaticMesh (Utilities|Struct|BreakS_CardInfo _returnvalue_2)) (.HP (Utilities|Struct|BreakS_CardInfo _returnvalue_2)) (.Damage (Utilities|Struct|BreakS_CardInfo _returnvalue_2)) (.Name (Utilities|Struct|BreakS_CardInfo _returnvalue_2))))))))))
  (Default|RefreshSlots (Variables|/Game/Dynamic/Blueprints/Player/BP_GS_GameState.BP_GS_GameState_C|GetTableRef (Variables|Default|GetBP_GameState%20Ref)))
  (Variables|Default|SetPlayerToMove (.OutItem (Utilities|Array|Random (Variables|Default|GetConnectedPlayersControllers)))))

(fn SpawnPlayer
  (params (PlayerController :type BP%20PC%20Player%20Controller%20Object%20Reference))
  (bind _returnvalue (Actor|GetActorOfClass "/Script/Engine.PlayerStart"))
  (bind _returnvalue_2 (Game|SpawnActorfromClass "/Game/Dynamic/Blueprints/Player/BP_P_Player.BP_P_Player_C" (Transformation|GetActorTransform _returnvalue) "Undefined" "MultiplyWithRoot" 0 0))
  (Pawn|Possess PlayerController _returnvalue_2)
  (Development|PrintString "PlayerSpawned"))

(fn CheckBothPlayersReady
  (if (== (Utilities|Array|Length (Variables|Default|GetReadyPlayers)) 2)
    (CallFunction|CreateTable)
    (Utilities|Time|ClearTimerbyFunctionName 0 "CheckBothPlayersReady")
    (return)))

(fn CreateTable
  (bind _returnvalue (Game|SpawnActorfromClass "/Game/Dynamic/Blueprints/Table/BP_Table.BP_Table_C" (LocalVariables|GetTableTransfrom) "Undefined" "MultiplyWithRoot" 0 0))
  (bind _asbp_gs_game_state (Utilities|Casting|CastToBP_GS_GameState (Game|GetGameState)))
  (bind _output_get (Variables|Default|SetBP_GameState%20Ref _asbp_gs_game_state))
  (Variables|/Game/Dynamic/Blueprints/Player/BP_GS_GameState.BP_GS_GameState_C|SetTableRef _output_get _returnvalue))

(fn CheckTablesReady
  (if (== (Variables|Default|GetReadyTables) 2)
    (CallFunction|StartGame)
    (Utilities|Time|ClearTimerbyFunctionName 0 "CheckTablesReady")))

(fn SetupPlayer0Cards
  (bind _nonusedcards (Variables|Default|GetNonUsedCards))
  (bind _output (Utilities|Array|Get(acopy) _nonusedcards))
  (for _index (range 0 3)
    (Utilities|Array|Add (Variables|Default|GetPlayer0Cards) _output)
    (Utilities|Array|RemoveItem (Variables|Default|GetNonUsedCards) _output)))

(fn SetupPlayer1Cards
  (bind _nonusedcards (Variables|Default|GetNonUsedCards))
  (bind _output (Utilities|Array|Get(acopy) _nonusedcards))
  (for _index (range 0 3)
    (Utilities|Array|Add (Variables|Default|GetPlayer1Cards) _output)
    (Utilities|Array|RemoveItem (Variables|Default|GetNonUsedCards) _output)))

(fn ManageCardAttack
  (params (Attacker :type Actor%20Object%20Reference) (Reciever :type Actor%20Object%20Reference))
  (bind _bp_gamestate_ref (Variables|Default|GetBP_GameState%20Ref))
  (bind _tableref (Variables|/Game/Dynamic/Blueprints/Player/BP_GS_GameState.BP_GS_GameState_C|GetTableRef _bp_gamestate_ref))
  (bind _slotsinfo (Variables|/Game/Dynamic/Blueprints/Table/BP_Table.BP_Table_C|GetSlotsInfo _tableref))
  (bind _cardinfo (Class|BPICardInterract|GetCardInfo(Message) Attacker))
  (LocalVariables|SetAttackerCardinfo _cardinfo)
  (bind _cardinfo_2 (Class|BPICardInterract|GetCardInfo(Message) Reciever))
  (LocalVariables|SetRecieverCardInfo _cardinfo_2)
  (bind _slotinfo (CallFunction|FindSlotInfobyCardName (.Name (Utilities|Struct|BreakS_CardInfo (LocalVariables|GetAttackerCardinfo)))))
  (if (.HasMoved? (Utilities|Struct|BreakS_SlotInfo _slotinfo))
    (Development|PrintString "CardHasmoved")
    (else
      (bind _output_get (LocalVariables|SetRecieverCardInfo (Utilities|Struct|MakeS_CardInfo (.StaticMesh (Utilities|Struct|BreakS_CardInfo (LocalVariables|GetRecieverCardInfo))) (- (.HP (Utilities|Struct|BreakS_CardInfo (LocalVariables|GetRecieverCardInfo))) (.Damage (Utilities|Struct|BreakS_CardInfo (LocalVariables|GetAttackerCardinfo)))) (.Damage (Utilities|Struct|BreakS_CardInfo (LocalVariables|GetRecieverCardInfo))) (.Name (Utilities|Struct|BreakS_CardInfo (LocalVariables|GetRecieverCardInfo))))))
      (bind _slotinfo_2 (CallFunction|FindSlotInfobyCardName (.Name (Utilities|Struct|BreakS_CardInfo _output_get))))
      (if (<= (.HP (Utilities|Struct|BreakS_CardInfo _output_get)) 0)
        (Utilities|Array|SetArrayElem _slotsinfo (.SlotIndex (Utilities|Struct|BreakS_SlotInfo _slotinfo_2)) (Utilities|Struct|MakeS_SlotInfo (.SlotIndex (Utilities|Struct|BreakS_SlotInfo _slotinfo_2)) (.OwningPlayerIndex (Utilities|Struct|BreakS_SlotInfo _slotinfo_2)) false (LocalVariables|GetRecieverCardInfo)))
        (else
          (Utilities|Array|SetArrayElem _slotsinfo (.SlotIndex (Utilities|Struct|BreakS_SlotInfo _slotinfo_2)) (Utilities|Struct|MakeS_SlotInfo (.SlotIndex (Utilities|Struct|BreakS_SlotInfo _slotinfo_2)) (.OwningPlayerIndex (Utilities|Struct|BreakS_SlotInfo _slotinfo_2)) true (LocalVariables|GetRecieverCardInfo)))))
      (bind _slotinfo_3 (CallFunction|FindSlotInfobyCardName (.Name (Utilities|Struct|BreakS_CardInfo (LocalVariables|GetAttackerCardinfo)))))
      (Utilities|Array|SetArrayElem _slotsinfo (.SlotIndex (Utilities|Struct|BreakS_SlotInfo _slotinfo_3)) (Utilities|Struct|MakeS_SlotInfo (.SlotIndex (Utilities|Struct|BreakS_SlotInfo _slotinfo_3)) (.OwningPlayerIndex (Utilities|Struct|BreakS_SlotInfo _slotinfo_3)) (.Occupied? (Utilities|Struct|BreakS_SlotInfo _slotinfo_3)) (LocalVariables|GetAttackerCardinfo) true))
      (Default|RefreshSlots _tableref))))

(fn FindSlotInfobyCardName
  (params (CardName :type Name))
  (for _array_element (Variables|/Game/Dynamic/Blueprints/Table/BP_Table.BP_Table_C|GetSlotsInfo (Variables|/Game/Dynamic/Blueprints/Player/BP_GS_GameState.BP_GS_GameState_C|GetTableRef (Variables|Default|GetBP_GameState%20Ref)))
    (if (== (.Name (Utilities|Struct|BreakS_CardInfo (.CardInfo (Utilities|Struct|BreakS_SlotInfo _array_element)))) CardName)
      (return _array_element))))

(fn ManageAttackCard
  (params (AttackerCardIndex :type Integer) (RecieverCardIndex :type Integer))
  (bind _bp_gamestate_ref (Variables|Default|GetBP_GameState%20Ref))
  (bind _bp_gamestate_ref_2 (Variables|Default|GetBP_GameState%20Ref))
  (bind _tableref (Variables|/Game/Dynamic/Blueprints/Player/BP_GS_GameState.BP_GS_GameState_C|GetTableRef _bp_gamestate_ref))
  (bind _tableref_2 (Variables|/Game/Dynamic/Blueprints/Player/BP_GS_GameState.BP_GS_GameState_C|GetTableRef _bp_gamestate_ref_2))
  (bind _slotsinfo (Variables|/Game/Dynamic/Blueprints/Table/BP_Table.BP_Table_C|GetSlotsInfo _tableref))
  (bind _output (Utilities|Array|Get(acopy) _slotsinfo AttackerCardIndex))
  (bind _output_2 (Utilities|Array|Get(acopy) _slotsinfo RecieverCardIndex))
  (bind (_slotindex _owningplayerindex _occupied_ _cardinfo) (Utilities|Struct|BreakS_SlotInfo _output))
  (bind (_slotindex_2 _owningplayerindex_2 _occupied__2 _cardinfo_2) (Utilities|Struct|BreakS_SlotInfo _output_2))
  (if (not (== AttackerCardIndex RecieverCardIndex))
    (if _occupied_
      (if _occupied__2
        (LocalVariables|SetAttackerCardInfo _cardinfo)
        (LocalVariables|SetRecieverCardInfo _cardinfo_2)
        (bind _slotinfo (CallFunction|FindSlotInfobyCardName (.Name (Utilities|Struct|BreakS_CardInfo (LocalVariables|GetRecieverCardInfo)))))
        (LocalVariables|SetRecieverSlotInfo _slotinfo)
        (bind _slotinfo_2 (CallFunction|FindSlotInfobyCardName (.Name (Utilities|Struct|BreakS_CardInfo (LocalVariables|GetAttackerCardInfo)))))
        (bind _output_get (LocalVariables|SetAttackerSlotInfo _slotinfo_2))
        (if (not (.HasMoved? (Utilities|Struct|BreakS_SlotInfo _output_get)))
          (bind _output_get_2 (LocalVariables|SetNewHP (- (.HP (Utilities|Struct|BreakS_CardInfo (LocalVariables|GetRecieverCardInfo))) (.Damage (Utilities|Struct|BreakS_CardInfo (LocalVariables|GetAttackerCardInfo))))))
          (LocalVariables|SetRecieverCardInfo (Utilities|Struct|MakeS_CardInfo (.StaticMesh (Utilities|Struct|BreakS_CardInfo (LocalVariables|GetRecieverCardInfo))) _output_get_2 (.Damage (Utilities|Struct|BreakS_CardInfo (LocalVariables|GetRecieverCardInfo))) (.Name (Utilities|Struct|BreakS_CardInfo (LocalVariables|GetRecieverCardInfo)))))
          (if (<= (LocalVariables|GetNewHP) 0)
            (Utilities|Array|SetArrayElem (Variables|/Game/Dynamic/Blueprints/Table/BP_Table.BP_Table_C|GetSlotsInfo (Variables|/Game/Dynamic/Blueprints/Player/BP_GS_GameState.BP_GS_GameState_C|GetTableRef (Variables|Default|GetBP_GameState%20Ref))) (.SlotIndex (Utilities|Struct|BreakS_SlotInfo (LocalVariables|GetRecieverSlotInfo))) (Utilities|Struct|MakeS_SlotInfo (.SlotIndex (Utilities|Struct|BreakS_SlotInfo (LocalVariables|GetRecieverSlotInfo))) (.OwningPlayerIndex (Utilities|Struct|BreakS_SlotInfo (LocalVariables|GetRecieverSlotInfo))) false (LocalVariables|GetRecieverCardInfo)))
            (else
              (Utilities|Array|SetArrayElem (Variables|/Game/Dynamic/Blueprints/Table/BP_Table.BP_Table_C|GetSlotsInfo (Variables|/Game/Dynamic/Blueprints/Player/BP_GS_GameState.BP_GS_GameState_C|GetTableRef (Variables|Default|GetBP_GameState%20Ref))) (.SlotIndex (Utilities|Struct|BreakS_SlotInfo (LocalVariables|GetRecieverSlotInfo))) (Utilities|Struct|MakeS_SlotInfo (.SlotIndex (Utilities|Struct|BreakS_SlotInfo (LocalVariables|GetRecieverSlotInfo))) (.OwningPlayerIndex (Utilities|Struct|BreakS_SlotInfo (LocalVariables|GetRecieverSlotInfo))) true (LocalVariables|GetRecieverCardInfo)))))
          (Utilities|Array|SetArrayElem (Variables|/Game/Dynamic/Blueprints/Table/BP_Table.BP_Table_C|GetSlotsInfo _tableref_2) (.SlotIndex (Utilities|Struct|BreakS_SlotInfo (LocalVariables|GetAttackerSlotInfo))) (Utilities|Struct|MakeS_SlotInfo (.SlotIndex (Utilities|Struct|BreakS_SlotInfo (LocalVariables|GetAttackerSlotInfo))) (.OwningPlayerIndex (Utilities|Struct|BreakS_SlotInfo (LocalVariables|GetAttackerSlotInfo))) (.Occupied? (Utilities|Struct|BreakS_SlotInfo (LocalVariables|GetAttackerSlotInfo))) (LocalVariables|GetAttackerCardInfo) true))
          (Default|RefreshSlots _tableref_2)
          (bind (_playerwonindex _playerwon_) (CallFunction|CheckPlayerWon))
          (if _playerwon_
            (CallFunction|ManagePlayerWon _playerwonindex)
            (elif (CallFunction|TurnEndedForplayer? (.OwningPlayerIndex (Utilities|Struct|BreakS_SlotInfo (Utilities|Array|Get(acopy) (Variables|/Game/Dynamic/Blueprints/Table/BP_Table.BP_Table_C|GetSlotsInfo (Variables|/Game/Dynamic/Blueprints/Player/BP_GS_GameState.BP_GS_GameState_C|GetTableRef (Variables|Default|GetBP_GameState%20Ref))) AttackerCardIndex))))
              (bind _array_element (Utilities|Array|ForEachLoopwithBreak (Variables|Default|GetConnectedPlayersControllers) :!label _label)
                (:LoopBody
                  (if (not (== (Variables|Default|GetPlayerToMove) _array_element))
                    (Variables|Default|SetPlayerToMove _array_element)
                    (for (_array_element_2 _array_index) (Variables|/Game/Dynamic/Blueprints/Table/BP_Table.BP_Table_C|GetSlotsInfo (Variables|/Game/Dynamic/Blueprints/Player/BP_GS_GameState.BP_GS_GameState_C|GetTableRef (Variables|Default|GetBP_GameState%20Ref)))
                      (Utilities|Array|SetArrayElem (Variables|/Game/Dynamic/Blueprints/Table/BP_Table.BP_Table_C|GetSlotsInfo (Variables|/Game/Dynamic/Blueprints/Player/BP_GS_GameState.BP_GS_GameState_C|GetTableRef (Variables|Default|GetBP_GameState%20Ref))) _array_index (Utilities|Struct|MakeS_SlotInfo (.SlotIndex (Utilities|Struct|BreakS_SlotInfo _array_element_2)) (.OwningPlayerIndex (Utilities|Struct|BreakS_SlotInfo _array_element_2)) (.Occupied? (Utilities|Struct|BreakS_SlotInfo _array_element_2)) (.CardInfo (Utilities|Struct|BreakS_SlotInfo _array_element_2))))
                      (goto _label Break))))))))))))

(fn TurnEndedForplayer?
  (params (Playerindex :type Integer))
  (for _array_element (Variables|/Game/Dynamic/Blueprints/Table/BP_Table.BP_Table_C|GetSlotsInfo (Variables|/Game/Dynamic/Blueprints/Player/BP_GS_GameState.BP_GS_GameState_C|GetTableRef (Variables|Default|GetBP_GameState%20Ref)))
    (if (== (.OwningPlayerIndex (Utilities|Struct|BreakS_SlotInfo _array_element)) Playerindex)
      (if (.Occupied? (Utilities|Struct|BreakS_SlotInfo _array_element))
        (Math|Integer|IncrementInt (LocalVariables|GetOccupiedSlots)
          (:%20%20
            _)))
      (if (.HasMoved? (Utilities|Struct|BreakS_SlotInfo _array_element))
        (Math|Integer|IncrementInt (LocalVariables|GetCardsMoved)))))
  (if (== (LocalVariables|GetOccupiedSlots) (LocalVariables|GetCardsMoved))
    (return true)
    (else
      (return false))))

(fn CheckPlayerWon
  (for _array_element (Variables|/Game/Dynamic/Blueprints/Table/BP_Table.BP_Table_C|GetSlotsInfo (Variables|/Game/Dynamic/Blueprints/Player/BP_GS_GameState.BP_GS_GameState_C|GetTableRef (Variables|Default|GetBP_GameState%20Ref)))
    (if (== (.OwningPlayerIndex (Utilities|Struct|BreakS_SlotInfo _array_element)) 0)
      (if (.Occupied? (Utilities|Struct|BreakS_SlotInfo _array_element))
        (Math|Integer|IncrementInt (LocalVariables|GetOccupiedSlotsPlayer0)))
      (elif (.Occupied? (Utilities|Struct|BreakS_SlotInfo _array_element))
        (Math|Integer|IncrementInt (LocalVariables|GetOccupiedSlotsPlayer1)))))
  (if (<= (LocalVariables|GetOccupiedSlotsPlayer0) 0)
    (return 1 true)
    (elif (<= (LocalVariables|GetOccupiedSlotsPlayer1) 0)
      (return 0 true)
      (else
        (return 67 false)))))

(fn ManagePlayerWon
  (params (PlayerWonIndex :type Integer))
  (for _array_element (Variables|Default|GetConnectedPlayersControllers)
    (if (== (Variables|/Game/Dynamic/Blueprints/Player/BP_PS_PlayerState.BP_PS_PlayerState_C|GetPlayerIndex (Variables|/Game/Dynamic/Blueprints/Player/BP_PC_PlayerController.BP_PC_PlayerController_C|GetAs%20BP%20PS%20Player%20State _array_element)) PlayerWonIndex)
      (Default|EndGame _array_element "YouWon")
      (else
        (Default|EndGame _array_element "YouLost")))))