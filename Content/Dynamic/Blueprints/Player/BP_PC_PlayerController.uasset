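; Player controller for a two-player card battle game, handling spawn and ready signals, card drafting, deck and end-game UI.
; SR_ events forward draft picks, slot assignments, attacks, abilities and spells to BP_GM_GameModeNew.
; ManageMouseClick traces under the cursor for BPI_CardInterract cards: an own card then an enemy card requests an attack, re-clicking requests an ability.
; OC_PickCardForSpell makes the next card click a spell target.
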(event Custom|SR_SpawnPlayer
  ;[0.15 0.15 0.15 0.5] Logic for game preparation
  (bind _asbp_gm_game_mode_new (Utilities|Casting|CastToBP_GM_GameModeNew (Game|GetGameMode)))
  (bind _output_get (Variables|Default|SetAs%20BP%20GM%20Game%20Mode _asbp_gm_game_mode_new))
  (Default|SpawnPlayer _output_get self))

(event Custom|SR_AttackCardRequest
  (params (Attacker :type Actor%20Object%20Reference) (Reciever :type Actor%20Object%20Reference))
  (Default|ManageCardAttackRequest (Variables|Default|GetAs%20BP%20GM%20Game%20Mode) Attacker Reciever self))

(event Custom|OC_OpenDeck
  (bind _self self)
  ;[0.15 0.15 0.15 0.5] Deck logic
  (Utilities|IsValid (Variables|Default|GetWBP_DeckRef)
    (:Is%20Valid
      (Widget|RemovefromParent (Variables|Default|GetWBP_DeckRef))
      (Variables|Default|SetWBP_DeckRef 0))
    (:Is%20Not%20Valid
      (bind _returnvalue (UserInterface|CreateWidget "/Game/Dynamic/UI/Widgets/InGame/WBP_Deck.WBP_Deck_C" _self _self))
      (bind _output_get (Variables|Default|SetWBP_DeckRef _returnvalue))
      (UserInterface|Viewport|AddtoViewport _output_get 0)
      (Input|SetInputModeGameandUI self _output_get "DoNotLock" false false)
      (Widget|SetFocus _output_get))))

(event Custom|SR_CardAssignedToSlot
  (params (CardInfo :type S%20Card%20Info%20Structure) (PlayerIndex :type Integer) (SlotIndex :type Integer))
  ;[0.15 0.15 0.15 0.5] Assigning cards to slots logic
  (Default|AssignCardtoSlot (Variables|Default|GetAs%20BP%20GM%20Game%20Mode) SlotIndex CardInfo PlayerIndex))

(event Custom|SR_CanIAssignCardToSlot?
  (params (ClickedSlotIndex :type Integer))
  ;[0.15 0.15 0.15 0.5] Assigning cards to slots logic
  (Default|CanIAssignCard? (Variables|Default|GetAs%20BP%20GM%20Game%20Mode) (Variables|/Game/Dynamic/Blueprints/Player/BP_PS_PlayerState.BP_PS_PlayerState_C|GetPlayerIndex (Variables|Default|GetAs%20BP%20PS%20Player%20State)) ClickedSlotIndex self))

(event Custom|SR_SpellManage
  (params (CardInfo :type S%20Card%20Info%20Structure))
  ;[0.15 0.15 0.15 0.5] Spells logic
  (Default|SpellManage (Variables|Default|GetAs%20BP%20GM%20Game%20Mode) self CardInfo))

(event Custom|OC_PickCardForSpell
  ;[0.15 0.15 0.15 0.5] Spells logic
  (Variables|Default|SetIsPickingCardForSpell? true))

(event Custom|SR_CardForSpellPicked
  (params (PickedCard :type S%20Card%20Info%20Structure))
  ;[0.15 0.15 0.15 0.5] Spells logic
  (Default|CardforSpellPicked (Variables|Default|GetAs%20BP%20GM%20Game%20Mode) PickedCard))

(event Custom|SR_RequestAbilityUse
  (params (CardInfo :type S%20Card%20Info%20Structure))
  (Default|ManageCardAbility (Variables|Default|GetAs%20BP%20GM%20Game%20Mode) CardInfo))

(event Custom|SR_RequestCardAttack
  (params (AttackerCardIndex :type Integer) (RecieverCardIndex :type Integer))
  ;[0.15 0.15 0.15 0.5] Card attacking logic
  (Default|ManageRequestCardAttack (Variables|Default|GetAs%20BP%20GM%20Game%20Mode) AttackerCardIndex RecieverCardIndex self))

(event Custom|SR_PlayerReady
  ;[0.15 0.15 0.15 0.5] Logic for game preparation
  (Default|PlayerReady (Variables|Default|GetAs%20BP%20GM%20Game%20Mode) self))

(event Custom|SR_TableReady
  ;[0.15 0.15 0.15 0.5] Logic for game preparation
  (Default|TableReady (Variables|Default|GetAs%20BP%20GM%20Game%20Mode)))

(event Custom|EndGame
  (params (EndGameText :type Text))
  ;[0.15 0.15 0.15 0.5] End game
  (bind _returnvalue (UserInterface|CreateWidget "/Game/Dynamic/UI/Widgets/InGame/WBP_EndGame.WBP_EndGame_C" self EndGameText))
  (UserInterface|Viewport|AddtoViewport _returnvalue 0)
  (Widget|SetFocus _returnvalue))

(event Custom|ShowPlayerCardsForDraft
  (params (CardInfo1 :type S%20Card%20Info%20Structure) (CardInfo2 :type S%20Card%20Info%20Structure))
  (bind _choicewidget (Variables|Default|GetChoiceWidget))
  (bind _carddraftactor (Variables|Default|GetCardDraftActor))
  ;[0.15 0.15 0.15 0.5] Drafting logic
  (bind _output_get (Variables|/Game/Dynamic/Blueprints/Cards/BP_CardDraftPosition.BP_CardDraftPosition_C|SetCardInfo1 (Variables|Default|GetCardDraftActor) CardInfo1))
  (bind _output_get_2 (Variables|/Game/Dynamic/Blueprints/Cards/BP_CardDraftPosition.BP_CardDraftPosition_C|SetCardInfo2 (Variables|Default|GetCardDraftActor) CardInfo2))
  (Variables|/Game/Dynamic/UI/Widgets/InGame/WBP_CardsChoice.WBP_CardsChoice_C|SetCardForDraft1 (Variables|Default|GetChoiceWidget) _output_get)
  (Variables|/Game/Dynamic/UI/Widgets/InGame/WBP_CardsChoice.WBP_CardsChoice_C|SetCardForDraft2 (Variables|Default|GetChoiceWidget) _output_get_2)
  (Variables|/Game/Dynamic/UI/Widgets/InGame/WBP_CardsChoice.WBP_CardsChoice_C|SetMat1 _choicewidget (Variables|/Game/Dynamic/Blueprints/Cards/BP_CardDraftPosition.BP_CardDraftPosition_C|GetCardMat1 _carddraftactor))
  (Variables|/Game/Dynamic/UI/Widgets/InGame/WBP_CardsChoice.WBP_CardsChoice_C|SetMat2 _choicewidget (Variables|/Game/Dynamic/Blueprints/Cards/BP_CardDraftPosition.BP_CardDraftPosition_C|GetCardMat2 _carddraftactor))
  (Utilities|FlowControl|Delay 0.1)
  (UserInterface|Viewport|AddtoViewport (Variables|Default|GetChoiceWidget) 0))

(event Custom|SR_CardPicked
  (params (Cardpicked :type S%20Card%20Info%20Structure))
  ;[0.15 0.15 0.15 0.5] Drafting logic
  (Default|CardPicked (Variables|Default|GetAs%20BP%20GM%20Game%20Mode) Cardpicked (Variables|/Game/Dynamic/Blueprints/Player/BP_PS_PlayerState.BP_PS_PlayerState_C|GetPlayerIndex (Variables|Default|GetAs%20BP%20PS%20Player%20State))))

(event Custom|SlotClicked
  (params (SlotIndex :type Integer))
  (bind _self self)
  ;[0.15 0.15 0.15 0.5] Assigning cards to slots logic
  (Utilities|IsValid (Variables|Default|GetWBP_DeckRef)
    (:Is%20Valid
      (Widget|RemovefromParent (Variables|Default|GetWBP_DeckRef))
      (Variables|Default|SetWBP_DeckRef 0))
    (:Is%20Not%20Valid
      (bind _returnvalue (UserInterface|CreateWidget "/Game/Dynamic/UI/Widgets/InGame/WBP_Deck.WBP_Deck_C" _self _self SlotIndex))
      (bind _output_get (Variables|Default|SetWBP_DeckRef _returnvalue))
      (UserInterface|Viewport|AddtoViewport _output_get 0)
      (Input|SetInputModeGameandUI self _output_get "DoNotLock" false false)
      (Widget|SetFocus _output_get))))

(event Custom|SR_DeckRequest
  ;[0.15 0.15 0.15 0.5] Deck logic
  (Default|RequestDeck (Variables|Default|GetAs%20BP%20GM%20Game%20Mode) self))

(event Input|EnhancedActionEvents|EnhancedInputActionIA_OpenDeck
  (params (ActionValue :type Boolean) (ElapsedSeconds :type Float%20%28double-precision%29) (TriggeredSeconds :type Float%20%28double-precision%29) (InputAction :type Input%20Action%20Object%20Reference :default "/Game/Dynamic/Input/IA_OpenDeck.IA_OpenDeck"))
  ;[0.15 0.15 0.15 0.5] Deck logic
  (:Started
    (CallFunction|SRDeckRequest)))

(event EventBeginPlay
  ;[0.15 0.15 0.15 0.5] Begin play logic
  (if (Pawn|IsLocalPlayerController)
    (CallFunction|SRSpawnPlayer)
    (Utilities|Time|SetTimerbyFunctionName 0 "TrySetPlayerReady" 0.02 true)
    (Variables|Default|SetbShowMouseCursor true)
    (Variables|Default|SetbEnableClickEvents true)
    (bind _returnvalue (Game|SpawnActorfromClass :Class "/Game/Dynamic/Blueprints/Cards/BP_CardDraftPosition.BP_CardDraftPosition_C" :SpawnTransform (Math|Transform|MakeTransform "-1000.000000,0.000000,0.000000") :CollisionHandlingOverride "Undefined" :TransformScaleMethod "MultiplyWithRoot" :Instigator 0))
    (Variables|Default|SetCardDraftActor _returnvalue)
    (bind _returnvalue_2 (UserInterface|CreateWidget :Class "/Game/Dynamic/UI/Widgets/InGame/WBP_CardsChoice.WBP_CardsChoice_C" :OwningPlayer self :Mat1 0 :Mat2 0))
    (Variables|Default|SetChoiceWidget _returnvalue_2)
    (Input|AddMappingContext (PlayerController|LocalPlayerSubsystems|GetEnhancedInputLocalPlayerSubsystem self) "/Game/Dynamic/Input/IMC_DafaultInput.IMC_DafaultInput" 0 "(bIgnoreAllPressedKeysUntilRelease=True,bForceImmediately=False,bNotifyUserSettings=False)")))

(event Input|MouseEvents|LeftMouseButton
  (params (Key :type Key%20Structure))
  (bind _lastclickedcard (Variables|Default|GetLastClickedCard))
  ;[0.15 0.15 0.15 0.5] Manage mouse clicking
  (:Pressed
    (CallFunction|ManageMouseClick)
    (Utilities|IsValid _lastclickedcard
      (:Is%20Valid
        (Class|BPICardInterract|CardClicked(Message) _lastclickedcard)))))

(fn ConstructionScript)

(fn NewFunction)

(fn OnRepasBPPSPlayerState
  (CallFunction|SRPlayerReady))

(fn TrySetPlayerReady
  (CallFunction|SRPlayerReady)
  (Utilities|Time|ClearTimerbyFunctionName 0 "TrySetPlayerReady"))

(fn SetLastClickedCard
  (params (HitActor :type Actor%20Object%20Reference))
  (Class|BPICardInterract|GetSlotIndex(Message) HitActor))

(fn ManageMouseClick
  (bind (_hitresult _returnvalue) (Game|Player|GetHitResultUnderCursorbyChannel "TraceTypeQuery1" true))
  (bind _hitactor (Collision|BreakHitResult _hitresult))
  (if _returnvalue
    (if (Utilities|DoesObjectImplementInterface _hitactor "/Game/Dynamic/Blueprints/Cards/Interface/BPI_CardInterract.BPI_CardInterract_C")
      (Utilities|IsValid (Variables|Default|GetLastClickedCard)
        (:Is%20Valid
          (Class|BPICardInterract|CardUnclicked(Message) (Variables|Default|GetLastClickedCard))
          (if (== (Variables|Default|GetLastClickedCard) _hitactor)
            (bind _cardinfo (Class|BPICardInterract|GetCardInfo(Message) (Variables|Default|GetLastClickedCard)))
            (CallFunction|SRRequestAbilityUse _cardinfo)
            (else
              (bind _output_get (Variables|Default|SetLastClickedCard _hitactor :!label _label))
              (bind _ownerplayerindex (Class|BPICardInterract|GetOwnerPlayerIndex(Message) _output_get))
              (if (Variables|Default|GetIsPickingCardForSpell?)
                (bind _cardinfo_2 (Class|BPICardInterract|GetCardInfo(Message) (Variables|Default|GetLastClickedCard)))
                (CallFunction|SRCardforSpellPicked _cardinfo_2)
                (Variables|Default|SetIsPickingCardForSpell? false)
                (elif (== _ownerplayerindex (Variables|/Game/Dynamic/Blueprints/Player/BP_PS_PlayerState.BP_PS_PlayerState_C|GetPlayerIndex (Variables|Default|GetAs%20BP%20PS%20Player%20State)))
                  (bind _slotindex (Class|BPICardInterract|GetSlotIndex(Message) (Variables|Default|GetLastClickedCard)))
                  (Variables|Default|SetLastClickedCardMineIndex _slotindex)
                  (Variables|Default|SetLastClickedAllieCard (Variables|Default|GetLastClickedCard))
                  (Variables|Default|SetHasSelectedCard true)
                  (return (Variables|Default|GetLastClickedCard))
                  (elif (Variables|Default|GetHasSelectedCard)
                    (bind _slotindex_2 (Class|BPICardInterract|GetSlotIndex(Message) (Variables|Default|GetLastClickedCard)))
                    (Variables|Default|SetLastClickedCardEnemyIndex _slotindex_2)
                    (CallFunction|SRRequestCardAttack (Variables|Default|GetLastClickedCardMineIndex) (Variables|Default|GetLastClickedCardEnemyIndex))
                    (bind _output_get_2 (Variables|Default|SetLastClickedEnemyCard (Variables|Default|GetLastClickedCard)))
                    (Variables|Default|SetHasSelectedCard false)
                    (return (Variables|Default|GetLastClickedCard))))))))
        (:Is%20Not%20Valid
          (goto _label))))))

(fn ManageLastClickedCard
  (params (LastClickedCard :type Actor%20Object%20Reference) (LastClickedCardMine :type Actor%20Object%20Reference) (LastClickedCardEnemy :type Actor%20Object%20Reference))
  (if (and (== LastClickedCard LastClickedCardEnemy) (Utilities|IsValid LastClickedCardMine))
    (bind _ownerplayerindex (Class|BPICardInterract|GetOwnerPlayerIndex(Message) LastClickedCard))
    (if (not (== _ownerplayerindex (Variables|/Game/Dynamic/Blueprints/Player/BP_PS_PlayerState.BP_PS_PlayerState_C|GetPlayerIndex (Variables|Default|GetAs%20BP%20PS%20Player%20State))))
      (CallFunction|AttackCard LastClickedCardMine LastClickedCardEnemy))))

(fn AttackCard
  (params (LastClickedCardMine :type Actor%20Object%20Reference) (LastClickedCardEnemy :type Actor%20Object%20Reference))
  (CallFunction|SRAttackCardRequest LastClickedCardMine LastClickedCardEnemy))

(fn MakeTransformforDraftposition
  (if (== (Variables|/Game/Dynamic/Blueprints/Player/BP_PS_PlayerState.BP_PS_PlayerState_C|GetPlayerIndex (Variables|Default|GetAs%20BP%20PS%20Player%20State)) 0)
    (return (Math|Transform|MakeTransform "-1000.000000,0.000000,0.000000"))
    (else
      (return (Math|Transform|MakeTransform "1000.000000,0.000000,0.000000")))))