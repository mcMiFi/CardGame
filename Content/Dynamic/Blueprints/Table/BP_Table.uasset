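; Card game table actor with two rows of four slots, showing the replicated board state as BP_Card actors.
; OnRep_SlotsInfo calls RefreshSlots to spawn, update or destroy cards, placing the local player's in the bottom row and others on top.
; A looping timer waits for controller and PlayerState, then reports ready to the server.
; Bottom-slot clicks request server card placement; older LocalCardVisuals spawning logic remains in disconnected nodes.
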(event OnClicked(Slot3)
  (params (TouchedComponent :type Primitive%20Component%20Object%20Reference) (ButtonPressed :type Key%20Structure :default "None"))
  (Development|PrintString "Hello")
  (Default|SRCanIAssignCardtoSlot? (Variables|Default|GetAs%20BP%20PC%20Player%20Controller) 3))

(event OnClicked(Slot0)
  (params (TouchedComponent :type Primitive%20Component%20Object%20Reference) (ButtonPressed :type Key%20Structure :default "None"))
  (Development|PrintString "Hello")
  (Default|SRCanIAssignCardtoSlot? (Variables|Default|GetAs%20BP%20PC%20Player%20Controller)))

(event OnClicked(Slot1)
  (params (TouchedComponent :type Primitive%20Component%20Object%20Reference) (ButtonPressed :type Key%20Structure :default "None"))
  (Development|PrintString "Hello")
  (Default|SRCanIAssignCardtoSlot? (Variables|Default|GetAs%20BP%20PC%20Player%20Controller) 1))

(event OnClicked(Slot2)
  (params (TouchedComponent :type Primitive%20Component%20Object%20Reference) (ButtonPressed :type Key%20Structure :default "None"))
  (Development|PrintString "Hello")
  (Default|SRCanIAssignCardtoSlot? (Variables|Default|GetAs%20BP%20PC%20Player%20Controller) 2))

(event Custom|RefreshSlots
  (for (_array_element _array_index) (Variables|Default|GetSlotsInfo)
    (if (.Occupied? (Utilities|Struct|BreakS_SlotInfo _array_element))
      (if (.ReturnValue (Utilities|Map|Find (Variables|Default|GetCardVisuals) _array_index))
        (CallFunction|UpdateLocalCards _array_element _array_index)
        (else
          (CallFunction|SpawnLocalCardforSlot _array_index _array_element)))
      (elif (.ReturnValue (Utilities|Map|Find (Variables|Default|GetCardVisuals) _array_index))
        (Actor|DestroyActor (.Value (Utilities|Map|Find (Variables|Default|GetCardVisuals) _array_index)))
        (Utilities|Map|Remove (Variables|Default|GetCardVisuals) _array_index)))))

(event EventBeginPlay
  (Utilities|Time|SetTimerbyFunctionName 0 "CheckTableReady" 0.02 true))

(fn ConstructionScript
  (Utilities|Array|Add (Variables|Default|GetBotSlots) (Variables|Default|GetSlot0))
  (Utilities|Array|Add (Variables|Default|GetBotSlots) (Variables|Default|GetSlot1))
  (Utilities|Array|Add (Variables|Default|GetBotSlots) (Variables|Default|GetSlot2))
  (Utilities|Array|Add (Variables|Default|GetBotSlots) (Variables|Default|GetSlot3))
  (Utilities|Array|Add (Variables|Default|GetTopSlots) (Variables|Default|GetSlot4))
  (Utilities|Array|Add (Variables|Default|GetTopSlots) (Variables|Default|GetSlot5))
  (Utilities|Array|Add (Variables|Default|GetTopSlots) (Variables|Default|GetSlot6))
  (Utilities|Array|Add (Variables|Default|GetTopSlots) (Variables|Default|GetSlot7)))

(fn OnRepSlotsInfo
  (CallFunction|RefreshSlots)
  (Development|PrintString "CLIENT REFRESHING SLOTS"))

(fn IsMyCard?
  (params (SlotInfo :type S%20Slot%20Info%20Structure))
  (if (== (Variables|/Game/Dynamic/Blueprints/Player/BP_PS_PlayerState.BP_PS_PlayerState_C|GetPlayerIndex (Variables|Default|GetAs%20BP%20PS%20Player%20State)) (.OwningPlayerIndex (Utilities|Struct|BreakS_SlotInfo SlotInfo)))
    (return true)
    (else
      (return false))))

(fn CheckTableReady
  (bind _asbp_pc_player_controller (Utilities|Casting|CastToBP_PC_PlayerController (Game|GetPlayerController 0)))
  (Variables|Default|SetAs%20BP%20PC%20Player%20Controller _asbp_pc_player_controller)
  (bind _asbp_ps_player_state (Utilities|Casting|CastToBP_PS_PlayerState (Variables|/Script/Engine.Controller|GetPlayerState _asbp_pc_player_controller)))
  (Variables|Default|SetAs%20BP%20PS%20Player%20State _asbp_ps_player_state)
  (Default|SRTableReady _asbp_pc_player_controller)
  (Utilities|Time|ClearTimerbyFunctionName 0 "CheckTableReady")
  (return))

(fn ManageSpawningOwnCards
  (params (SlotInfo :type S%20Slot%20Info%20Structure))
  (bind (_slotindex _owningplayerindex _occupied_ _cardinfo) (Utilities|Struct|BreakS_SlotInfo SlotInfo))
  (bind (_slotindex_2 _owningplayerindex_2 _occupied__2 _cardinfo_2) (Utilities|Struct|BreakS_SlotInfo SlotInfo))
  (bind _returnvalue (- _slotindex_2 4))
  (if (> _slotindex 3)
    (if _occupied__2
      (if (not (Utilities|Map|Contains (Variables|Default|GetLocalCardVisuals) _returnvalue))
        (bind _returnvalue_2 (Utilities|GetDataTableRow (Variables|Default|GetDT_Cards) (.Name (Utilities|Struct|BreakS_CardInfo _cardinfo_2)))
          (:then
            (bind _returnvalue_3 (Game|SpawnActorfromClass "/Game/Dynamic/Blueprints/Cards/BP_Card.BP_Card_C" (Math|Transform|MakeTransform (Transformation|GetWorldLocation (Utilities|Array|Get(acopy) (Variables|Default|GetBotSlots) _returnvalue))) "Undefined" "MultiplyWithRoot" 0 0 (Utilities|Struct|MakeS_CardInfo (.StaticMesh (Utilities|Struct|BreakS_CardInfo _returnvalue_2)) (.HP (Utilities|Struct|BreakS_CardInfo _returnvalue_2)) (.Damage (Utilities|Struct|BreakS_CardInfo _returnvalue_2)) (.Name (Utilities|Struct|BreakS_CardInfo _returnvalue_2)) (.IsSplash? (Utilities|Struct|BreakS_CardInfo _returnvalue_2)) (.IsSpell? (Utilities|Struct|BreakS_CardInfo _returnvalue_2)) (.Picture (Utilities|Struct|BreakS_CardInfo _returnvalue_2))) _owningplayerindex_2 0))
            (Utilities|Map|Add (Variables|Default|GetLocalCardVisuals) _returnvalue _returnvalue_3)))))
    (elif _occupied_
      (if (not (Utilities|Map|Contains (Variables|Default|GetLocalCardVisuals) _slotindex))
        (bind _returnvalue_4 (Utilities|GetDataTableRow (Variables|Default|GetDT_Cards) (.Name (Utilities|Struct|BreakS_CardInfo _cardinfo)))
          (:then
            (bind _returnvalue_5 (Game|SpawnActorfromClass "/Game/Dynamic/Blueprints/Cards/BP_Card.BP_Card_C" (Math|Transform|MakeTransform (Transformation|GetWorldLocation (Utilities|Array|Get(acopy) (Variables|Default|GetBotSlots) _slotindex))) "Undefined" "MultiplyWithRoot" 0 0 (Utilities|Struct|MakeS_CardInfo (.StaticMesh (Utilities|Struct|BreakS_CardInfo _returnvalue_4)) (.HP (Utilities|Struct|BreakS_CardInfo _returnvalue_4)) (.Damage (Utilities|Struct|BreakS_CardInfo _returnvalue_4)) (.Name (Utilities|Struct|BreakS_CardInfo _returnvalue_4)) (.IsSplash? (Utilities|Struct|BreakS_CardInfo _returnvalue_4)) (.IsSpell? (Utilities|Struct|BreakS_CardInfo _returnvalue_4)) (.Picture (Utilities|Struct|BreakS_CardInfo _returnvalue_4))) _owningplayerindex 0))
            (Utilities|Map|Add (Variables|Default|GetLocalCardVisuals) _slotindex _returnvalue_5)))))))

(fn ManageSpawningEnemyCards
  (params (SlotInfo :type S%20Slot%20Info%20Structure))
  (bind (_slotindex _owningplayerindex _occupied_ _cardinfo) (Utilities|Struct|BreakS_SlotInfo SlotInfo))
  (bind (_slotindex_2 _owningplayerindex_2 _occupied__2 _cardinfo_2) (Utilities|Struct|BreakS_SlotInfo SlotInfo))
  (if (> _slotindex 3)
    (if _occupied__2
      (CallFunction|ManageEnemyOccupiedSlots _slotindex_2 _owningplayerindex_2 _cardinfo_2))
    (elif _occupied_
      (if (not (Utilities|Map|Contains (Variables|Default|GetLocalCardVisuals) (+ _slotindex 4)))
        (bind _returnvalue (Utilities|GetDataTableRow (Variables|Default|GetDT_Cards) (.Name (Utilities|Struct|BreakS_CardInfo _cardinfo)))
          (:then
            (bind _returnvalue_2 (Game|SpawnActorfromClass "/Game/Dynamic/Blueprints/Cards/BP_Card.BP_Card_C" (Math|Transform|MakeTransform (Transformation|GetWorldLocation (Utilities|Array|Get(acopy) (Variables|Default|GetTopSlots) _slotindex))) "Undefined" "MultiplyWithRoot" 0 0 (Utilities|Struct|MakeS_CardInfo (.StaticMesh (Utilities|Struct|BreakS_CardInfo _returnvalue)) (.HP (Utilities|Struct|BreakS_CardInfo _returnvalue)) (.Damage (Utilities|Struct|BreakS_CardInfo _returnvalue)) (.Name (Utilities|Struct|BreakS_CardInfo _returnvalue)) (.IsSplash? (Utilities|Struct|BreakS_CardInfo _returnvalue)) (.IsSpell? (Utilities|Struct|BreakS_CardInfo _returnvalue)) (.Picture (Utilities|Struct|BreakS_CardInfo _returnvalue))) _owningplayerindex 0))
            (Utilities|Map|Add (Variables|Default|GetLocalCardVisuals) (+ _slotindex 4) _returnvalue_2)))))))

(fn ManageEnemyOccupiedSlots
  (params (SlotIndex :type Integer%20%28by%20ref%29) (OwningPlayerIndex :type Integer) (S_CardInfo :type S%20Card%20Info%20Structure%20%28by%20ref%29))
  (bind _returnvalue (- SlotIndex 4))
  (if (not (Utilities|Map|Contains (Variables|Default|GetLocalCardVisuals) SlotIndex))
    (bind _returnvalue_2 (Utilities|GetDataTableRow (Variables|Default|GetDT_Cards) (.Name (Utilities|Struct|BreakS_CardInfo S_CardInfo)))
      (:then
        (bind _returnvalue_3 (Game|SpawnActorfromClass "/Game/Dynamic/Blueprints/Cards/BP_Card.BP_Card_C" (Math|Transform|MakeTransform (Transformation|GetWorldLocation (Utilities|Array|Get(acopy) (Variables|Default|GetTopSlots) _returnvalue))) "Undefined" "MultiplyWithRoot" 0 0 (Utilities|Struct|MakeS_CardInfo (.StaticMesh (Utilities|Struct|BreakS_CardInfo _returnvalue_2)) (.HP (Utilities|Struct|BreakS_CardInfo _returnvalue_2)) (.Damage (Utilities|Struct|BreakS_CardInfo _returnvalue_2)) (.Name (Utilities|Struct|BreakS_CardInfo _returnvalue_2)) (.IsSplash? (Utilities|Struct|BreakS_CardInfo _returnvalue_2)) (.IsSpell? (Utilities|Struct|BreakS_CardInfo _returnvalue_2)) (.Picture (Utilities|Struct|BreakS_CardInfo _returnvalue_2))) OwningPlayerIndex 0))
        (Utilities|Map|Add (Variables|Default|GetLocalCardVisuals) (+ _returnvalue 4) _returnvalue_3)))))

(fn ManageDeadCard
  (for (_array_element _array_index) (Variables|Default|GetSlotsInfo)
    (if (and (not (.Occupied? (Utilities|Struct|BreakS_SlotInfo _array_element))) (Utilities|Map|Contains (Variables|Default|GetLocalCardVisuals) (CallFunction|GetLocalCardIndex _array_index)))
      (Actor|DestroyActor (.Value (Utilities|Map|Find (Variables|Default|GetLocalCardVisuals) (CallFunction|GetLocalCardIndex _array_index))))
      (Utilities|Map|Remove (Variables|Default|GetLocalCardVisuals) (CallFunction|GetLocalCardIndex _array_index)))))

(fn GetLocalCardIndex
  (params (SlotIndex :type Integer))
  (if (== (Variables|/Game/Dynamic/Blueprints/Player/BP_PS_PlayerState.BP_PS_PlayerState_C|GetPlayerIndex (Variables|Default|GetAs%20BP%20PS%20Player%20State)) 0)
    (return SlotIndex)
    (else
      (return (- 7 SlotIndex)))))

(fn GetLocalPlayerIndex
  (return (Variables|/Game/Dynamic/Blueprints/Player/BP_PS_PlayerState.BP_PS_PlayerState_C|GetPlayerIndex (Variables|Default|GetAs%20BP%20PS%20Player%20State))))

(fn GetVisualTransformSlot
  (params (GlobalSlotIndex :type Integer))
  (LocalVariables|SetRowIndex (Math|Integer|%(Integer) GlobalSlotIndex 4))
  (bind _output_get (LocalVariables|SetOwnerindex (.OwningPlayerIndex (Utilities|Struct|BreakS_SlotInfo (Utilities|Array|Get(acopy) (Variables|Default|GetSlotsInfo) GlobalSlotIndex)))))
  (if (== _output_get (CallFunction|GetLocalPlayerIndex))
    (return (Math|Transform|MakeTransform (Transformation|GetWorldLocation (Utilities|Array|Get(acopy) (Variables|Default|GetBotSlots) (LocalVariables|GetRowIndex)))))
    (else
      (return (Math|Transform|MakeTransform (Transformation|GetWorldLocation (Utilities|Array|Get(acopy) (Variables|Default|GetTopSlots) (LocalVariables|GetRowIndex))))))))

(fn SpawnLocalCardforSlot
  (params (GlobalSlotIndex :type Integer) (SlotInfo :type S%20Slot%20Info%20Structure))
  (bind (_slotindex _owningplayerindex _occupied_ _cardinfo) (Utilities|Struct|BreakS_SlotInfo SlotInfo))
  (bind _returnvalue (Game|SpawnActorfromClass "/Game/Dynamic/Blueprints/Cards/BP_Card.BP_Card_C" (CallFunction|GetVisualTransformSlot GlobalSlotIndex) "Undefined" "MultiplyWithRoot" 0 GlobalSlotIndex _cardinfo _owningplayerindex 0))
  (Utilities|Map|Add (Variables|Default|GetCardVisuals) GlobalSlotIndex _returnvalue))

(fn UpdateLocalCards
  (params (SlotInfo :type S%20Slot%20Info%20Structure) (GlobalSlotIndex :type Integer))
  (bind _cardvisuals (Variables|Default|GetCardVisuals))
  (bind _value (Utilities|Map|Find _cardvisuals GlobalSlotIndex))
  (Class|BPICardInterract|SetCardInfo(Message) _value (.CardInfo (Utilities|Struct|BreakS_SlotInfo SlotInfo)))
  (Default|RefreshVisuals _value))

(fn ManageSlotsHitboxes
  (params (On? :type Boolean))
  (if On?
    (Collision|SetCollisionEnabled (Variables|Default|GetSlot0) "QueryOnly")
    (Collision|SetCollisionEnabled (Variables|Default|GetSlot1) "QueryOnly")
    (Collision|SetCollisionEnabled (Variables|Default|GetSlot2) "QueryOnly")
    (Collision|SetCollisionEnabled (Variables|Default|GetSlot3) "QueryOnly")
    (else
      (Collision|SetCollisionEnabled (Variables|Default|GetSlot0) "NoCollision")
      (Collision|SetCollisionEnabled (Variables|Default|GetSlot1) "NoCollision")
      (Collision|SetCollisionEnabled (Variables|Default|GetSlot2) "NoCollision")
      (Collision|SetCollisionEnabled (Variables|Default|GetSlot3) "NoCollision"))))